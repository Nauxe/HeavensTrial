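; Base enemy that fires projectiles at the player while AI perception senses them.
; A looping ShootPlayer timer, paused and unpaused by perception updates, spawns BP_LX_BaseProjectile at the Arrow, targeting the tracked pawn.
; TakeDamage delegates to BPCLXDamageComponent, which also feeds the health bar widget and has its events bound in the construction script.
; Death pauses shooting and ragdolls the mesh, while block, parry and damage responses only print debug strings.
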(event `self.ReceiveBeginPlay`
  (`KismetSystemLibrary.K2_SetTimer` null "ShootPlayer" (`self.ShootDelay`) true)
  (`KismetSystemLibrary.K2_PauseTimer` null "ShootPlayer")
  (bind _returnvalue (`|CreateWidget` "/Game/DamageSystem/W_LX_Healthbar.W_LX_Healthbar_C" null (`self.BPC_LX_DamageComponent`)))
  (`WidgetComponent.SetWidget` (`self.HealthBar`) _returnvalue))

(event `self.AIPerception.OnTargetPerceptionUpdated`
  (params (Actor :type "Actor Object Reference") (Stimulus :type "AIStimulus Structure"))
  (bind _returnvalue (`GameplayStatics.GetPlayerPawn` 0))
  ; Track pawn
  (if (== Actor _returnvalue)
    (bind _output_get (set `self.IsTracking` (`.bSuccessfullySensed` (break `AIStimulus` Stimulus))))
    (if _output_get
      (set `self.CurrentTrackedPawn` _returnvalue)
      (`KismetSystemLibrary.K2_UnPauseTimer` null "ShootPlayer")
      (else
        (`KismetSystemLibrary.K2_PauseTimer` null "ShootPlayer")))))

(event `Death`
  (`KismetSystemLibrary.PrintString` "enemy death")
  (`KismetSystemLibrary.K2_PauseTimer` null "ShootPlayer")
  (`PrimitiveComponent.SetSimulatePhysics` (`self.SkeletalMesh`) true))

(event `Block`
  (`KismetSystemLibrary.PrintString` "blocked on enemy"))

(event `Parry`
  (`KismetSystemLibrary.PrintString` "parried on enemy"))

(event `DamageResponse`
  (params (DamageResponse :type "/Game/DamageSystem/E_LX_DamageResponse Enum" :default "NewEnumerator0"))
  (`KismetSystemLibrary.PrintString` (`|GetEnumeratorNameAsString` DamageResponse)))

(fn `ShootPlayer`
  (`|SpawnActorFromClass` "/Game/Blueprints/Enemy/BP_LX_BaseProjectile.BP_LX_BaseProjectile_C" (`SceneComponent.K2_GetComponentToWorld` (`self.Arrow`)) "Undefined" "MultiplyWithRoot" self (`self.ProjectileSpeed`) (`self.CurrentTrackedPawn`) null))

(fn `TakeDamage`
  (params (DamageInfo :type "/Game/DamageSystem/S_LX_DamageInfo Structure"))
  (returns (WasDamaged :type Boolean))
  (bind _wasdamaged (`/Game/DamageSystem/BPI_LX_Damagable.TakeDamage` (`self.BPC_LX_DamageComponent`) DamageInfo))
  (return _wasdamaged))

(fn `UserConstructionScript`
  (add `/Game/DamageSystem/BPC_LX_DamageComponent.OnDeath` (`self.BPC_LX_DamageComponent`) (`|CreateDelegate` :!event `Death`))
  (add `/Game/DamageSystem/BPC_LX_DamageComponent.OnBlock` (`self.BPC_LX_DamageComponent`) (`|CreateDelegate` :!event `Block`))
  (add `/Game/DamageSystem/BPC_LX_DamageComponent.OnParry` (`self.BPC_LX_DamageComponent`) (`|CreateDelegate` :!event `Parry`))
  (add `/Game/DamageSystem/BPC_LX_DamageComponent.OnDamageResponse` (`self.BPC_LX_DamageComponent`) (`|CreateDelegate` :!event `DamageResponse`)))