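; Base enemy projectile that flies at a set Speed toward a Target actor and destroys itself on overlapping it, with no damage logic here.
; The construction script copies Speed into the ProjectileMovement initial and max speeds.
; On BeginPlay, a valid Target sets a one-time straight-line velocity, without homing.
; The owner ignore-when-moving call passes false, so the Box does not ignore its owner despite the graph comment.
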(event `self.ReceiveBeginPlay`
  ; Initialize direction of projectile and ignore collision with enemy class
  (`self.Target`
    (:`then`
      (`self.RotateToTarget`)
      (`PrimitiveComponent.IgnoreActorWhenMoving` (`self.Box`) (`self.GetOwner`) false))
    (:`else`)))

(event `self.ReceiveActorBeginOverlap`
  (params (OtherActor :type "Actor Object Reference"))
  (if (== OtherActor (`self.Target`))
    (`self.K2_DestroyActor`)))

(fn `RotateToTarget`
  (set `MovementComponent.Velocity` (* (`KismetMathLibrary.GetDirectionUnitVector` (`self.K2_GetActorLocation`) (`self.K2_GetActorLocation` (`self.Target`))) (`self.Speed`)) (`self.ProjectileMovement`)))

(fn `UserConstructionScript`
  (bind _projectilemovement (`self.ProjectileMovement`))
  (set `ProjectileMovementComponent.InitialSpeed` (`self.Speed`) _projectilemovement)
  (set `ProjectileMovementComponent.MaxSpeed` (`self.Speed`) _projectilemovement))