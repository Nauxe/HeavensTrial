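; Damage component that tracks health and death for its owning actor and resolves incoming hits as damage, block or parry.
; TakeDamage routes DamageInfo through the CanBeDamaged multi-exit check, where parrying requires an active, permitted block.
; Hits reduce Health and fire response and death events, while blocks and parries fire their own events.
; Heal clamps to MaxHealth, and BeginPlay caches a VRPawn owner that these graphs never use.
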(event `self.ReceiveBeginPlay`
  (bind _asvrpawn (cast `/Game/Blueprints/VRPawn` (`self.GetOwner`)))
  (set `self.Player` _asvrpawn))

(fn `GetCurrentHealth`
  (returns (Health :type "Float (double-precision)"))
  (return (`self.Health`)))

(fn `GetMaxHealth`
  (returns (MaxHealth :type "Float (double-precision)"))
  (return (`self.MaxHealth`)))

(fn `Heal`
  (params (Amount :type "Float (double-precision)"))
  (returns (NewHealth :type "Float (double-precision)"))
  (if (not (`self.IsDead`))
    (bind _output_get (set `self.Health` (`KismetMathLibrary.FClamp` (+ Amount (`self.Health`)) 0.0 (`self.MaxHealth`)))))
  (return _output_get))

(fn `TakeDamage`
  (params (DamageInfo :type "/Game/DamageSystem/S_LX_DamageInfo Structure"))
  (returns (WasDamaged :type Boolean))
  (bind (_amount _damagetype _damageresponse _canbeblocked _canbeparried) (break `/Game/DamageSystem/S_LX_DamageInfo` DamageInfo))
  (if (not (`self.IsDead`))
    (`self.CanBeDamaged` _canbeblocked _canbeparried
      (:`NoDamage`
        (`KismetSystemLibrary.PrintString` "NotDamaged")
        (return false))
      (:`DoDamage`
        (bind _output_get (set `self.Health` (- (`self.Health`) _amount)))
        (`KismetSystemLibrary.PrintString` (`|GetEnumeratorNameAsString` _damageresponse))
        (`self.OnDamageResponse` _damageresponse)
        (if (<= _output_get 0.0)
          (set `self.IsDead` true)
          (`self.OnDeath`))
        (return true))
      (:`BlockDamage`
        (`KismetSystemLibrary.PrintString` "Blocked!")
        (`self.OnBlock`))
      (:`ParryDamage`
        (`KismetSystemLibrary.PrintString` "Parried!")
        (`self.OnParry`)))
    (return false)))